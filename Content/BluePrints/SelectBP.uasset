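; SelectBP is a gaze-dwell selectable element with a widget showing a text label and a progress bar.
; Each Tick it consumes the IsSelect flag, playing SelectTimeLine while the flag keeps being set and reversing it otherwise, with Percent driving the bar.
; When the timeline finishes at full Percent, it passes its SelectIndex to SelectElement on the first "Select"-tagged actor, cast to MultiSelectBP.
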(event EventTick
  (params (DeltaSeconds :type Float%20%28single-precision%29))
  ;[1 1 1] Tick処理
  (if (Variables|Default|GetisSelect)
    (Variables|Default|SetisSelect false) ; わざとここで選択済みフラグを倒す
    (bind _percent (Timeline|SelectTimeLine Play)
      (:Update
        (Variables|Default|Setpercent _percent)
        (Progress|SetPercent (Variables|/Game/UI/SelectUI.SelectUI_C|GetSelectProgressBar (.AsSelect%20UI (Utilities|Casting|CastToSelectUI (UserInterface|GetUserWidgetObject (Variables|Default|GetWidget))))) (Variables|Default|Getpercent)) ; プログレスバーにセット
      )
      (:Finished
        (if (>= (Variables|Default|Getpercent) 1.0)
          ;;[0 0.9093 1] 視線入力による選択処理
          (bind _outactors (Actor|GetAllActorswithTag "Select"))
          (bind _asmulti_select_bp (Utilities|Casting|CastToMultiSelectBP (Utilities|Array|Get(acopy) _outactors)))
          (Default|SelectElement _asmulti_select_bp (Variables|Default|GetselectIndex)))))
    (else
      (Timeline|SelectTimeLine Reverse))))

(fn ConstructionScript)

(fn SetText
  (params (Text :type String))
  ;[1 1 1] ラベルをセット
  (Rendering|Components|TextRender|SetText (Variables|/Game/UI/SelectUI.SelectUI_C|GetSelectText (.AsSelect%20UI (Utilities|Casting|CastToSelectUI (UserInterface|GetUserWidgetObject (Variables|Default|GetWidget))))) (Utilities|Text|ToText(String) Text)))