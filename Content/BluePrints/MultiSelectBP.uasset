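; Multiple-choice menu actor that presents three SelectBP child-actor options and reports the chosen one to the game manager.
; BeginPlay sets hard-coded Japanese text and indices on the second and third options, leaving the first untouched.
; SelectElement shows only the matching option, hides all after a short delay, then calls SelectMulti once on the GM-tagged BP_GM.
; ShowSelect and HideSelect toggle all three options' visibility.
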(event Custom|SelectElement
  (params (SelectIndex :type Integer))
  ;[1 1 1] 選択イベント
  (Utilities|FlowControl|Sequence
    (:then_0
      ;;[0.9948 1 0] 選択したもの以外を非表示
      (CallFunction|Select (Variables|Default|GetSelectBP) SelectIndex))
    (:then_1
      (CallFunction|Select (Variables|Default|GetSelectBP1) SelectIndex))
    (:then_2
      (CallFunction|Select (Variables|Default|GetSelectBP2) SelectIndex))
    (:then_3
      (Utilities|FlowControl|Delay 0.5)
      (CallFunction|HideSelect) ; 全選択肢を非表示
      (bind _outactors (Actor|GetAllActorswithTag "GM"))
      (bind _asbp_gm (Utilities|Casting|CastToBP_GM (Utilities|Array|Get(acopy) _outactors)))
      (Utilities|FlowControl|DoOnce false
        (:Completed
          (Default|SelectMulti _asbp_gm SelectIndex) ; 選択したことを通知
        )))))

(event EventBeginPlay
  ;[1 1 1] 初期化イベント
  (Utilities|FlowControl|Sequence
    (:then_0
      (bind _asselect_bp (Utilities|Casting|CastToSelectBP (Variables|/Script/Engine.ChildActorComponent|GetChildActor (Variables|Default|GetSelectBP1))))
      (Default|SetText _asselect_bp "ユニティちゃんと夜のスノボする")
      (Variables|/Game/BluePrints/SelectBP.SelectBP_C|SetselectIndex _asselect_bp 1))
    (:then_1
      (bind _asselect_bp_2 (Utilities|Casting|CastToSelectBP (Variables|/Script/Engine.ChildActorComponent|GetChildActor (Variables|Default|GetSelectBP2))))
      (Default|SetText _asselect_bp_2 "我を忘れるほどスノボをする")
      (Variables|/Game/BluePrints/SelectBP.SelectBP_C|SetselectIndex _asselect_bp_2 2))))

(fn ConstructionScript)

(fn ShowSelect
  ;[1 1 1] 全選択肢を表示
  (Utilities|FlowControl|Sequence
    (:then_0
      (Rendering|SetVisibility (Variables|Default|GetSelectBP) true false))
    (:then_1
      (Rendering|SetVisibility (Variables|Default|GetSelectBP1) true false))
    (:then_2
      (Rendering|SetVisibility (Variables|Default|GetSelectBP2) true false))))

(fn HideSelect
  ;[1 1 1] 全選択肢を非表示
  (Utilities|FlowControl|Sequence
    (:then_0
      (Rendering|SetVisibility (Variables|Default|GetSelectBP) false false))
    (:then_1
      (Rendering|SetVisibility (Variables|Default|GetSelectBP1) false false))
    (:then_2
      (Rendering|SetVisibility (Variables|Default|GetSelectBP2) false false))))

(fn Select
  (params (selectBP :type Child%20Actor%20Component%20Object%20Reference) (selectIndex :type Integer))
  ;[1 1 1] 選択したもの以外を非表示に
  (Rendering|SetVisibility selectBP (== (Variables|/Game/BluePrints/SelectBP.SelectBP_C|GetselectIndex (.AsSelect%20BP (Utilities|Casting|CastToSelectBP (Variables|/Script/Engine.ChildActorComponent|GetChildActor selectBP)))) selectIndex) false))