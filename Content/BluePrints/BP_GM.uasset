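; Game manager for a VR conversation with Unity-chan, sequencing her voice lines and the player's response prompts.
; Plays intro lines, then shows a nod yes/no prompt on the MotionControllerPawn; either answer gets its own reply before a shared line opens the gaze-driven MultiSelectBP choices.
; Any gaze choice triggers one closing line.
; PlayVoice pairs audio with five vowel lip-sync curves on the character, with delays timed from sound duration.
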(event Custom|SELECT_YES
  ;[1 1 1] ボイス再生
  ;;[0 0.8168 1] YESのボイス再生
  (CallFunction|PlayVoice "/Game/Sound/Voice/UnityChan/univ1126.univ1126" "/Game/Assets/UnityChan/crs/LipSyncData/Lips1126MTH_A.Lips1126MTH_A" "/Game/Assets/UnityChan/crs/LipSyncData/Lips1126MTH_I.Lips1126MTH_I" "/Game/Assets/UnityChan/crs/LipSyncData/Lips1126MTH_U.Lips1126MTH_U" "/Game/Assets/UnityChan/crs/LipSyncData/Lips1126MTH_E.Lips1126MTH_E" "/Game/Assets/UnityChan/crs/LipSyncData/Lips1126MTH_O.Lips1126MTH_O")
  (Utilities|FlowControl|Delay (+ (Variables|/Script/Engine.SoundBase|GetDuration (Variables|/Script/Engine.AudioComponent|GetSound (Variables|Default|GetUnityChanVoice))) 0.5))
  (CallFunction|PlayVoice "/Game/Sound/Voice/UnityChan/univ1340.univ1340" "/Game/Assets/UnityChan/crs/LipSyncData/Lips1340MTH_A.Lips1340MTH_A" "/Game/Assets/UnityChan/crs/LipSyncData/Lips1340MTH_I.Lips1340MTH_I" "/Game/Assets/UnityChan/crs/LipSyncData/Lips1340MTH_U.Lips1340MTH_U" "/Game/Assets/UnityChan/crs/LipSyncData/Lips1340MTH_E.Lips1340MTH_E" "/Game/Assets/UnityChan/crs/LipSyncData/Lips1340MTH_O.Lips1340MTH_O")
  (Utilities|FlowControl|Delay (Variables|/Script/Engine.SoundBase|GetDuration (Variables|/Script/Engine.AudioComponent|GetSound (Variables|Default|GetUnityChanVoice))))
  ;;[0 0.3791 1] 選択肢表示
  (bind _outactors (Actor|GetAllActorswithTag "Select"))
  (bind _asmulti_select_bp (Utilities|Casting|CastToMultiSelectBP (Utilities|Array|Get(acopy) _outactors)))
  (Default|ShowSelect _asmulti_select_bp)
  (bind _outactors_2 (Actor|GetAllActorswithTag "Player"))
  (Variables|/Game/VirtualRealityBP/Blueprints/MotionControllerPawn.MotionControllerPawn_C|SetisSelect (.AsMotion%20Controller%20Pawn (Utilities|Casting|CastToMotionControllerPawn (Utilities|Array|Get(acopy) _outactors_2))) true))

(event Custom|SELECT_NO
  ;[1 1 1] ボイス再生
  ;;[1 0.1147 0] NOのボイス再生
  (CallFunction|PlayVoice "/Game/Sound/Voice/UnityChan/univ1095.univ1095" "/Game/Assets/UnityChan/crs/LipSyncData/Lips1095MTH_A.Lips1095MTH_A" "/Game/Assets/UnityChan/crs/LipSyncData/Lips1095MTH_I.Lips1095MTH_I" "/Game/Assets/UnityChan/crs/LipSyncData/Lips1095MTH_U.Lips1095MTH_U" "/Game/Assets/UnityChan/crs/LipSyncData/Lips1095MTH_E.Lips1095MTH_E" "/Game/Assets/UnityChan/crs/LipSyncData/Lips1095MTH_O.Lips1095MTH_O")
  (Utilities|FlowControl|Delay (+ (Variables|/Script/Engine.SoundBase|GetDuration (Variables|/Script/Engine.AudioComponent|GetSound (Variables|Default|GetUnityChanVoice))) 0.5))
  (CallFunction|PlayVoice "/Game/Sound/Voice/UnityChan/univ1340.univ1340" "/Game/Assets/UnityChan/crs/LipSyncData/Lips1340MTH_A.Lips1340MTH_A" "/Game/Assets/UnityChan/crs/LipSyncData/Lips1340MTH_I.Lips1340MTH_I" "/Game/Assets/UnityChan/crs/LipSyncData/Lips1340MTH_U.Lips1340MTH_U" "/Game/Assets/UnityChan/crs/LipSyncData/Lips1340MTH_E.Lips1340MTH_E" "/Game/Assets/UnityChan/crs/LipSyncData/Lips1340MTH_O.Lips1340MTH_O")
  (Utilities|FlowControl|Delay (Variables|/Script/Engine.SoundBase|GetDuration (Variables|/Script/Engine.AudioComponent|GetSound (Variables|Default|GetUnityChanVoice))))
  ;;[0 0.3791 1] 選択肢表示
  (bind _outactors (Actor|GetAllActorswithTag "Select"))
  (bind _asmulti_select_bp (Utilities|Casting|CastToMultiSelectBP (Utilities|Array|Get(acopy) _outactors)))
  (Default|ShowSelect _asmulti_select_bp)
  (bind _outactors_2 (Actor|GetAllActorswithTag "Player"))
  (Variables|/Game/VirtualRealityBP/Blueprints/MotionControllerPawn.MotionControllerPawn_C|SetisSelect (.AsMotion%20Controller%20Pawn (Utilities|Casting|CastToMotionControllerPawn (Utilities|Array|Get(acopy) _outactors_2))) true))

(event Custom|SelectMulti
  (params (SelectIndex :type Integer))
  ;[1 1 1] ボイス再生
  (CallFunction|PlayVoice "/Game/Sound/Voice/UnityChan/univ1119.univ1119" "/Game/Assets/UnityChan/crs/LipSyncData/Lips1119MTH_A.Lips1119MTH_A" "/Game/Assets/UnityChan/crs/LipSyncData/Lips1119MTH_I.Lips1119MTH_I" "/Game/Assets/UnityChan/crs/LipSyncData/Lips1119MTH_U.Lips1119MTH_U" "/Game/Assets/UnityChan/crs/LipSyncData/Lips1119MTH_E.Lips1119MTH_E" "/Game/Assets/UnityChan/crs/LipSyncData/Lips1119MTH_O.Lips1119MTH_O")
  (Utilities|FlowControl|Delay (Variables|/Script/Engine.SoundBase|GetDuration (Variables|/Script/Engine.AudioComponent|GetSound (Variables|Default|GetUnityChanVoice)))))

(event EventBeginPlay
  (Utilities|FlowControl|Delay 2.0)
  ;[1 1 1] ボイス再生
  (CallFunction|PlayVoice "/Game/Sound/Voice/UnityChan/univ0041.univ0041" "/Game/Assets/UnityChan/crs/LipSyncData/Lips0041MTH_A.Lips0041MTH_A" "/Game/Assets/UnityChan/crs/LipSyncData/Lips0041MTH_I.Lips0041MTH_I" "/Game/Assets/UnityChan/crs/LipSyncData/Lips0041MTH_U.Lips0041MTH_U" "/Game/Assets/UnityChan/crs/LipSyncData/Lips0041MTH_E.Lips0041MTH_E" "/Game/Assets/UnityChan/crs/LipSyncData/Lips0041MTH_O.Lips0041MTH_O")
  (Utilities|FlowControl|Delay (+ (Variables|/Script/Engine.SoundBase|GetDuration (Variables|/Script/Engine.AudioComponent|GetSound (Variables|Default|GetUnityChanVoice))) 0.5))
  (CallFunction|PlayVoice "/Game/Sound/Voice/UnityChan/univ0043.univ0043" "/Game/Assets/UnityChan/crs/LipSyncData/Lips0043MTH_A.Lips0043MTH_A" "/Game/Assets/UnityChan/crs/LipSyncData/Lips0043MTH_I.Lips0043MTH_I" "/Game/Assets/UnityChan/crs/LipSyncData/Lips0043MTH_U.Lips0043MTH_U" "/Game/Assets/UnityChan/crs/LipSyncData/Lips0043MTH_E.Lips0043MTH_E" "/Game/Assets/UnityChan/crs/LipSyncData/Lips0043MTH_O.Lips0043MTH_O")
  (Utilities|FlowControl|Delay (+ (Variables|/Script/Engine.SoundBase|GetDuration (Variables|/Script/Engine.AudioComponent|GetSound (Variables|Default|GetUnityChanVoice))) 0.5))
  (CallFunction|PlayVoice "/Game/Sound/Voice/UnityChan/univ0026.univ0026" "/Game/Assets/UnityChan/crs/LipSyncData/Lips0026MTH_A.Lips0026MTH_A" "/Game/Assets/UnityChan/crs/LipSyncData/Lips0026MTH_I.Lips0026MTH_I" "/Game/Assets/UnityChan/crs/LipSyncData/Lips0026MTH_U.Lips0026MTH_U" "/Game/Assets/UnityChan/crs/LipSyncData/Lips0026MTH_E.Lips0026MTH_E" "/Game/Assets/UnityChan/crs/LipSyncData/Lips0026MTH_O.Lips0026MTH_O")
  (Utilities|FlowControl|Delay (Variables|/Script/Engine.SoundBase|GetDuration (Variables|/Script/Engine.AudioComponent|GetSound (Variables|Default|GetUnityChanVoice))))
  ;;[1 0.9267 0] うなずきアクション表示
  (bind _outactors (Actor|GetAllActorswithTag "Player"))
  (Default|ShowSelect (.AsMotion%20Controller%20Pawn (Utilities|Casting|CastToMotionControllerPawn (Utilities|Array|Get(acopy) _outactors)))))

(fn ConstructionScript)

(fn PlayVoice
  (params (NewSound :type Sound%20Base%20Object%20Reference) (LipA :type Curve%20Float%20Object%20Reference) (LipI :type Curve%20Float%20Object%20Reference) (LipU :type Curve%20Float%20Object%20Reference) (LipE :type Curve%20Float%20Object%20Reference) (LipO :type Curve%20Float%20Object%20Reference))
  (Audio|Components|Audio|SetSound (Variables|Default|GetUnityChanVoice) NewSound)
  (bind _outactors (Actor|GetAllActorswithTag "UnityChan"))
  (Default|PlayLip (.AsCandy%20Rock%20Star%20Blueprint (Utilities|Casting|CastToCandyRockStar_Blueprint (Utilities|Array|Get(acopy) _outactors))) (Variables|/Script/Engine.SoundBase|GetDuration (Variables|/Script/Engine.AudioComponent|GetSound (Variables|Default|GetUnityChanVoice))) LipA LipI LipU LipE LipO)
  (Audio|Components|Audio|Play (Variables|Default|GetUnityChanVoice) 0.0))