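; CandyRockStar character Blueprint that adds lip sync, random blinking and player gaze tracking, all driven through its CRS_AnimatinoBP anim instance.
; PlayLip stores five vowel float curves and runs a timeline in reverse from the voice duration, sampling them by elapsed time into lip morph targets.
; A randomized BeginPlay loop plays a timeline on the eye-smile morphs to blink.
; Tick feeds the Player-tagged MotionControllerPawn's camera position into LookAtLocation.
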(event Custom|PlayLip
  (params (Duration :type Float%20%28single-precision%29) (LipACurveFloat :type Curve%20Float%20Object%20Reference) (LipICurveFloat :type Curve%20Float%20Object%20Reference) (LipUCurveFloat :type Curve%20Float%20Object%20Reference) (LipECurveFloat :type Curve%20Float%20Object%20Reference) (LipOCurveFloat :type Curve%20Float%20Object%20Reference))
  ;[0 0.335 1] リップシンクイベント
  (Utilities|FlowControl|Sequence
    (:then_0
      (Variables|Default|SetVoiceDuration Duration)
      (bind _liptime (Timeline|LipsyncTimeLine SetNewTime)
        (:Update
          (Variables|Default|SetNowVoiceTime (- (Variables|Default|GetVoiceDuration) _liptime))
          (Default|SetLipsyncMorphTarget (.AsCRS%20Animatino%20BP (Utilities|Casting|CastToCRS_AnimatinoBP (Components|SkeletalMesh|GetAnimInstance (Variables|SkeletalMeshActor|GetSkeletalMeshComponent)))) (Math|Curves|GetFloatValue (Variables|Default|GetLipACurve) (Variables|Default|GetNowVoiceTime)) (Math|Curves|GetFloatValue (Variables|Default|GetLipICurve) (Variables|Default|GetNowVoiceTime)) (Math|Curves|GetFloatValue (Variables|Default|GetLipUCurve) (Variables|Default|GetNowVoiceTime)) (Math|Curves|GetFloatValue (Variables|Default|GetLipECurve) (Variables|Default|GetNowVoiceTime)) (Math|Curves|GetFloatValue (Variables|Default|GetLipOCurve) (Variables|Default|GetNowVoiceTime))))))
    (:then_1
      (Variables|Default|SetLipACurve LipACurveFloat))
    (:then_2
      (Variables|Default|SetLipICurve LipICurveFloat))
    (:then_3
      (Variables|Default|SetLipUCurve LipUCurveFloat))
    (:then_4
      (Variables|Default|SetLipECurve LipECurveFloat))
    (:then_5
      (Variables|Default|SetLipOCurve LipOCurveFloat))
    (:then_6
      (Timeline|LipsyncTimeLine Reverse))))

(event EventBeginPlay
  ;[0.8838 1 0] 目パチ判定
  (if (> (Math|Random|RandomInteger 50) 45) :!label _label ; 乱数が一定値の場合、目パチさせる
    ;[1 1 1] 目パチ処理
    (bind _morph (Timeline|MorphTimeLine PlayFromStart)
      (:Update
        (bind _ascrs_animatino_bp (Utilities|Casting|CastToCRS_AnimatinoBP (Components|SkeletalMesh|GetAnimInstance (Variables|SkeletalMeshActor|GetSkeletalMeshComponent))))
        (Components|SkeletalMesh|SetMorphTarget _ascrs_animatino_bp "EYE_SMILE1" _morph)
        (Components|SkeletalMesh|SetMorphTarget _ascrs_animatino_bp "EYE_SMILE2" _morph))
      (:Finished
        (goto _label)))
    (else
      (Utilities|FlowControl|Delay 0.5)
      (goto _label))))

(event EventTick
  (params (DeltaSeconds :type Float%20%28single-precision%29))
  ;[0 1 0.1765] カメラの位置をセット
  (bind _outactors (Actor|GetAllActorswithTag "Player"))
  (Variables|/Game/Assets/UnityChan/crs/Animation/CRS_AnimatinoBP.CRS_AnimatinoBP_C|SetLookAtLocation (.AsCRS%20Animatino%20BP (Utilities|Casting|CastToCRS_AnimatinoBP (Components|SkeletalMesh|GetAnimInstance (Variables|SkeletalMeshActor|GetSkeletalMeshComponent)))) (Transformation|GetWorldLocation (Variables|/Game/VirtualRealityBP/Blueprints/MotionControllerPawn.MotionControllerPawn_C|GetCamera (.AsMotion%20Controller%20Pawn (Utilities|Casting|CastToMotionControllerPawn (Utilities|Array|Get(acopy) _outactors)))))))

(fn ConstructionScript)