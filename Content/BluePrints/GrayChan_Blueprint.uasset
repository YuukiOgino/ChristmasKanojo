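; GrayChan character Blueprint that blinks at random and feeds the player's position to its animation for look-at.
; A loop from BeginPlay rolls a random chance, either retrying after a short delay or playing a timeline that drives both eye-close morph targets through GrayChan_AnimationBP.
; Each Tick copies the camera location of the Player-tagged MotionControllerPawn into the AnimBP's LookAtLocation.
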(event EventBeginPlay
  ;[0.8838 1 0] 目パチ判定
  (if (> (Math|Random|RandomInteger 50) 45) :!label _label ; 乱数が一定値の場合、目パチさせる
    ;[1 1 1] 目パチ処理
    (bind _morph (Timeline|MorphTimeLint PlayFromStart)
      (:Update
        (bind _asgray_chan_animation_bp (Utilities|Casting|CastToGrayChan_AnimationBP (Components|SkeletalMesh|GetAnimInstance (Variables|SkeletalMeshActor|GetSkeletalMeshComponent))))
        (Components|SkeletalMesh|SetMorphTarget _asgray_chan_animation_bp "Eye_Close_L" _morph)
        (Components|SkeletalMesh|SetMorphTarget _asgray_chan_animation_bp "Eye_Close_R" _morph))
      (:Finished
        (goto _label)))
    (else
      (Utilities|FlowControl|Delay 0.5)
      (goto _label))))

(event EventTick
  (params (DeltaSeconds :type Float%20%28single-precision%29))
  (bind _outactors (Actor|GetAllActorswithTag "Player"))
  (Variables|/Game/Assets/GrayChan/Animations/GrayChan_AnimationBP.GrayChan_AnimationBP_C|SetLookAtLocation (.AsGray%20Chan%20Animation%20BP (Utilities|Casting|CastToGrayChan_AnimationBP (Components|SkeletalMesh|GetAnimInstance (Variables|SkeletalMeshActor|GetSkeletalMeshComponent)))) (Transformation|GetWorldLocation (Variables|/Game/VirtualRealityBP/Blueprints/MotionControllerPawn.MotionControllerPawn_C|GetCamera (.AsMotion%20Controller%20Pawn (Utilities|Casting|CastToMotionControllerPawn (Utilities|Array|Get(acopy) _outactors)))))))

(fn ConstructionScript)