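; ActionBPSpawn is a spawner actor that creates an ActionBP instance and relays a yes or no choice to it.
; Select spawns the action at the root component's location and rotation at half scale and stores the reference.
; Yes and No check that the reference is valid, call YesSelect or NoSelect on it, then trigger Remove.
; Remove destroys the spawned actor after a short delay and clears the reference.
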(event Custom|Remove
  (Utilities|FlowControl|Delay 1.0)
  (Actor|DestroyActor (Variables|Default|GetSpawnActionBP))
  (Variables|Default|SetSpawnActionBP 0))

(fn ConstructionScript)

(fn Select
  (bind _defaultsceneroot (Variables|Default|GetDefaultSceneRoot))
  (bind _returnvalue (Game|SpawnActorfromClass "/Game/BluePrints/ActionBP.ActionBP_C" (Math|Transform|MakeTransform (Transformation|GetWorldLocation _defaultsceneroot) (Transformation|GetWorldRotation _defaultsceneroot) "0.500000,0.500000,0.500000") "Undefined" 0 0))
  (Variables|Default|SetSpawnActionBP _returnvalue))

(fn Yes
  (bind _spawnactionbp (Variables|Default|GetSpawnActionBP))
  (Utilities|IsValid _spawnactionbp
    (:Is%20Valid
      (Default|YesSelect _spawnactionbp)
      (CallFunction|Remove))))

(fn No
  (bind _spawnactionbp (Variables|Default|GetSpawnActionBP))
  (Utilities|IsValid _spawnactionbp
    (:Is%20Valid
      (Default|NoSelect _spawnactionbp)
      (CallFunction|Remove))))