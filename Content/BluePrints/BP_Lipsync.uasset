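; BP_Lipsync is an experimental lip-sync Blueprint that estimates vowel formants from a fixed sound wave, Univ1340.
; Every Tick, it passes GetAmplitude output to GetFormant, with bin spacing set by sample rate over window size.
; GetFormant scans for local peaks, converting indices to frequencies for F1 and F2, gated by an IsFindFirst flag.
; It returns both as a Vector2D, which Tick currently leaves unused.
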(event EventBeginPlay)

(event Collision|EventActorBeginOverlap
  (params (OtherActor :type Actor%20Object%20Reference)))

(event EventTick
  (params (DeltaSeconds :type Float%20%28single-precision%29))
  (bind _outamplitudes (Class|SoundVisualizationStatics|GetAmplitude "/Game/Sound/Voice/UnityChan/univ1340.univ1340" 0 0.0 0.0))
  (CallFunction|GetFormant (/ 4.41e+04 1024.0) _outamplitudes))

(fn ConstructionScript)

(fn GetFormant
  (params (df :type Float%20%28single-precision%29) (input :type Array%20of%20Floats%20%28single-precision%29))
  (bind _index (Utilities|FlowControl|ForLoopwithBreak 1 (- (Utilities|Array|Length input) 1) :!label _label)
    (:LoopBody
      (if (and (> (Utilities|Array|Get(acopy) input _index) (Utilities|Array|Get(acopy) input (- _index 1))) (> (Utilities|Array|Get(acopy) input _index) (Utilities|Array|Get(acopy) input (+ _index 1))))
        (if (LocalVariables|GetisFindFirst)
          (LocalVariables|Setf1 (* df (Math|Conversions|ToFloat(Integer) _index)))
          (LocalVariables|SetisFindFirst true)
          (else
            (LocalVariables|Setf2 (* df (Math|Conversions|ToFloat(Integer) _index)))
            (goto _label Break)))))
    (:Completed
      (return (Math|Vector2D|MakeVector2D (LocalVariables|Getf1) (LocalVariables|Getf2))))))