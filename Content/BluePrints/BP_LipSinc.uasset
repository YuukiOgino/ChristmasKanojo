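; Unfinished lip-sync Actor Blueprint that begins LPC-based formant analysis of an array of sample values.
; GetFormantIndices applies a Hamming window, zeroes the endpoints, scales by the peak magnitude, then accumulates autocorrelation values for lags up to just past the LPC order.
; It stops there: no LPC coefficients or formants are computed, and the zero-valued return node is never reached.
; The event graph and construction script are empty.
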(event EventBeginPlay)

(event Collision|EventActorBeginOverlap
  (params (OtherActor :type Actor%20Object%20Reference)))

(event EventTick
  (params (DeltaSeconds :type Float%20%28single-precision%29)))

(fn ConstructionScript)

(fn GetFormantIndices
  (params (input :type Array%20of%20Floats%20%28single-precision%29))
  (bind _r (LocalVariables|Getr))
  (LocalVariables|Setinputlist input)
  (LocalVariables|Setn (Utilities|Array|Length (LocalVariables|Getinputlist)))
  (LocalVariables|Setorder (Variables|Default|GetlpcOrder))
  (for _index (range 1 (- (LocalVariables|Getn) 1))
    (LocalVariables|Seti _index)
    (Utilities|Array|SetArrayElem (LocalVariables|Getinputlist) (LocalVariables|Geti) (* (Utilities|Array|Get(acopy) (LocalVariables|Getinputlist) (LocalVariables|Geti)) (- 0.54 (* 0.46 (Math|Trig|Cos(Radians) (/ (* 2.0 (Math|Trig|GetPI) (Math|Conversions|ToFloat(Integer) (LocalVariables|Geti))) (Math|Conversions|ToFloat(Integer) (- (LocalVariables|Getn) 1)))))))))
  (Utilities|Array|SetArrayElem (LocalVariables|Getinputlist) 0 0.0)
  (Utilities|Array|SetArrayElem (LocalVariables|Getinputlist) (- (LocalVariables|Getn) 1) 0.0)
  (for _array_element (LocalVariables|Getinputlist)
    (if (> _array_element (LocalVariables|Getmax))
      (LocalVariables|Setmax _array_element))
    (if (< _array_element (LocalVariables|Getmin))
      (LocalVariables|Setmin _array_element)))
  (LocalVariables|Setmax (Math|Float|Absolute(Float) (LocalVariables|Getmax)))
  (LocalVariables|Setmin (Math|Float|Absolute(Float) (LocalVariables|Getmin)))
  (if (> (LocalVariables|Getmax) (LocalVariables|Getmin))
    (LocalVariables|Setfactor (/ 1.0 (LocalVariables|Getmax)))
    (elif (< (LocalVariables|Getmax) (LocalVariables|Getmin))
      (LocalVariables|Setfactor (/ 1.0 (LocalVariables|Getmin)))))
  (for (_array_element_2 _array_index) (LocalVariables|Getinputlist)
    (Utilities|Array|SetArrayElem (LocalVariables|Getinputlist) _array_index (* _array_element_2 (LocalVariables|Getfactor))))
  (for _index_2 (range 0 (+ (LocalVariables|Getorder) 1))
    (Utilities|Array|Add _r 0.0)
    (for (_ _array_index_2) (LocalVariables|Getinputlist)
      (Utilities|Array|SetArrayElem _r _index_2 (+ (* (Utilities|Array|Get(acopy) (LocalVariables|Getinputlist) _array_index_2) (Utilities|Array|Get(acopy) (LocalVariables|Getinputlist) (+ _array_index_2 _index_2))) (Utilities|Array|Get(acopy) _r _index_2))))))